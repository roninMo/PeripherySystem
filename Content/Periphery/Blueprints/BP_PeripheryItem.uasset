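; BP_PeripheryItem is a test item that responds to a character's periphery detection through periphery interface events.
; It receives enter and exit events for three detection types: radius, cone and trace.
; Each handler only prints a keyed debug message naming the item and the source character, with no other behavior or construction logic.
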(event EventWithinPlayerTracePeriphery
  (params (SourceCharacter :type Actor%20Object%20Reference) (PeripheryType :type EPeripheryType%20Enum :default "EPT_None"))
  ;[0 0.5885 0.1856 1 45] Periphery Object Interface Functions
  ;;[0 0.776 0.2594] Periphery Trace
  (Development|PrintString (Utilities|String|Append (Utilities|GetDisplayName self) " object inside " (Utilities|GetDisplayName SourceCharacter) "'s periphery trace") true true "(R=0.000000,G=1.000000,B=0.282915,A=1.000000)" 2.0 "objectTrace_inside"))

(event EventOutsideOfPlayerTracePeriphery
  (params (SourceCharacter :type Actor%20Object%20Reference) (PeripheryType :type EPeripheryType%20Enum :default "EPT_None"))
  ;[0 0.5885 0.1856 1 45] Periphery Object Interface Functions
  ;;[0 0.776 0.2594] Periphery Trace
  (Development|PrintString (Utilities|String|Append (Utilities|GetDisplayName self) " object outside of " (Utilities|GetDisplayName SourceCharacter) "'s periphery trace") true true "(R=0.000000,G=1.000000,B=0.282915,A=1.000000)" 2.0 "objectTrace_outside"))

(event EventOutsideOfPlayerRadiusPeriphery
  (params (SourceCharacter :type Actor%20Object%20Reference) (PeripheryType :type EPeripheryType%20Enum :default "EPT_None"))
  ;[0 0.5885 0.1856 1 45] Periphery Object Interface Functions
  ;;[0 0.776 0.2594] Periphery Radius
  (Development|PrintString (Utilities|String|Append (Utilities|GetDisplayName self) " object exited " (Utilities|GetDisplayName SourceCharacter) "'s radius") true true "(R=0.000000,G=1.000000,B=0.282915,A=1.000000)" 2.0 "objectRadius_outside"))

(event EventWithinPlayerRadiusPeriphery
  (params (SourceCharacter :type Actor%20Object%20Reference) (PeripheryType :type EPeripheryType%20Enum :default "EPT_None"))
  ;[0 0.5885 0.1856 1 45] Periphery Object Interface Functions
  ;;[0 0.776 0.2594] Periphery Radius
  (Development|PrintString (Utilities|String|Append (Utilities|GetDisplayName self) " object inside " (Utilities|GetDisplayName SourceCharacter) "'s radius") true true "(R=0.000000,G=1.000000,B=0.282915,A=1.000000)" 2.0 "objectRadius_inside"))

(event EventOutsideOfConePeriphery
  (params (SourceCharacter :type Actor%20Object%20Reference) (PeripheryType :type EPeripheryType%20Enum :default "EPT_None"))
  ;[0 0.5885 0.1856 1 45] Periphery Object Interface Functions
  ;;[0 0.776 0.2594] Periphery Cone
  (Development|PrintString (Utilities|String|Append (Utilities|GetDisplayName self) " object exited " (Utilities|GetDisplayName SourceCharacter) "'s periphery cone") true true "(R=0.000000,G=1.000000,B=0.282915,A=1.000000)" 2.0 "objectCone_outside"))

(event EventWithinPlayerConePeriphery
  (params (SourceCharacter :type Actor%20Object%20Reference) (PeripheryType :type EPeripheryType%20Enum :default "EPT_None"))
  ;[0 0.5885 0.1856 1 45] Periphery Object Interface Functions
  ;;[0 0.776 0.2594] Periphery Cone
  (Development|PrintString (Utilities|String|Append (Utilities|GetDisplayName self) " object inside " (Utilities|GetDisplayName SourceCharacter) "'s periphery cone") true true "(R=0.000000,G=1.000000,B=0.282915,A=1.000000)" 2.0 "objectCone_inside"))

(fn ConstructionScript)